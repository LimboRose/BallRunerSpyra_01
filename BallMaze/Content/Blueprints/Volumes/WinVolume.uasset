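; WinVolume is a trigger volume that ends a level once the player enters its box with no BP_Crystal actors left.
; CheckAnyCrystals counts remaining crystals and prints either congratulations or the shortfall.
; The current level's position in the LevelNames array decides the outcome: the last prints a win message and quits after a delay.
; Otherwise LoadNextLevel streams the following entry through LoadLevelInstance at the origin, rather than opening it.
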(event `self.Box.OnComponentBeginOverlap`
  (params (OverlappedComponent :type "PrimitiveComponent Object Reference") (OtherActor :type "Actor Object Reference") (OtherComp :type "PrimitiveComponent Object Reference") (OtherBodyIndex :type Integer) (bFromSweep :type Boolean) (SweepResult :type "HitResult Structure (by ref)"))
  (`/Game/Blueprints/Libraries/ML_Actors.IsPlayer` OtherActor
    (:`IsPlayer`
      (bind _crystals (`self.CheckAnyCrystals`))
      (if _crystals
        (bind _islast (`self.CompleteLevel`))
        (if _islast
          (`KismetSystemLibrary.PrintString` "Super, Wygrałes")
          (`KismetSystemLibrary.Delay` 3.0)
          (`KismetSystemLibrary.QuitGame` null "Quit")
          (else
            (`self.LoadNextLevel`)))))))

(fn `CheckAnyCrystals`
  (returns (Crystals :type Boolean))
  (bind _outactors (`GameplayStatics.GetAllActorsOfClass` "/Game/Blueprints/Actors/Collectables/BP_Crystal.BP_Crystal_C"))
  (bind _returnvalue (`KismetArrayLibrary.Array_Length` _outactors))
  (if (== _returnvalue 0)
    (`KismetSystemLibrary.PrintString` "Congratulations, you have found all crystals!")
    (return true)
    (else
      (`KismetSystemLibrary.PrintString` (`KismetStringLibrary.Conv_IntToString` _returnvalue))
      (`KismetSystemLibrary.PrintString` "I am sorry but there are still crystals to be found")
      (return false))))

(fn `CompleteLevel`
  (returns (isLast :type Boolean))
  (bind _index (`self.GetCurrentLevelIndex`))
  (bind _islast (`self.IsLastLevel` _index))
  (return _islast))

(fn `GetCurrentLevelIndex`
  (returns (Index :type Integer))
  (bind _returnvalue (`GameplayStatics.GetCurrentLevelName` true))
  (return (`KismetArrayLibrary.Array_Find` (`self.LevelNames`) (`KismetStringLibrary.Conv_StringToName` _returnvalue))))

(fn `IsLastLevel`
  (params (Index :type Integer))
  (returns (isLast :type Boolean))
  (return (== (`KismetArrayLibrary.Array_LastIndex` (`self.LevelNames`)) Index)))

(fn `LoadNextLevel`
  (bind _levelnames (`self.LevelNames`))
  (bind _returnvalue (`GameplayStatics.GetCurrentLevelName` true))
  (`LevelStreamingKismet.LoadLevelInstance` (`KismetStringLibrary.Conv_NameToString` (`|GetArrayItem` _levelnames (+ (`KismetArrayLibrary.Array_Find` _levelnames (`KismetStringLibrary.Conv_StringToName` _returnvalue)) 1)))))

(fn `UserConstructionScript`)