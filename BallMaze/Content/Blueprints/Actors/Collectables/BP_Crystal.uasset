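; BP_Crystal is a collectable crystal that gets sucked into the player and disappears when its collision radius is overlapped.
; On overlap it records its start location, then a timeline drives Wsysanko to move it toward the player pawn's live position, shrinking it and fading its point light.
; The actor destroys itself when the timeline finishes.
; The player-pawn check is unconnected, so any overlapping actor triggers the pickup.
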(event `self.CollisionRadius.OnComponentBeginOverlap`
  (params (OverlappedComponent :type "PrimitiveComponent Object Reference") (OtherActor :type "Actor Object Reference") (OtherComp :type "PrimitiveComponent Object Reference") (OtherBodyIndex :type Integer) (bFromSweep :type Boolean) (SweepResult :type "HitResult Structure (by ref)"))
  (bind _pointlight (`self.PointLight`))
  (bind _output_get (`self.Collectable Location`))
  (bind (_direction _smoothlerpalpha _lightanimation) (`Timeline|TL_BlendAlpha` :`NewTime` 0.7)
    (:`Update`
      (`self.Wsysanko` (`KismetMathLibrary.VLerp` _output_get (`self.K2_GetActorLocation` (`GameplayStatics.GetPlayerPawn` 0)) _smoothlerpalpha) (`KismetMathLibrary.VLerp` (`self.GetActorScale3D`) (0.0 0.0 0.0) _smoothlerpalpha) _pointlight (`KismetMathLibrary.Lerp` (`LightComponentBase.Intensity` _pointlight) 0.0 _lightanimation)))
    (:`Finished`
      (`self.K2_DestroyActor`))))

(fn `Collectable Location`
  (returns (Output_Get :type "Vector Structure"))
  (bind _output_get (set `self.LerpStartLocation` (`self.K2_GetActorLocation`)))
  (return _output_get))

(fn `CollectableLocation`
  (returns (Output_Get :type "Vector Structure"))
  (bind _output_get (set `self.LerpStartLocation` (`self.K2_GetActorLocation`)))
  (return _output_get))

(fn `ScalingAnimation`
  (params (Alpha :type "Float (double-precision)"))
  (returns (ReturnValue :type "Vector Structure"))
  (return (`KismetMathLibrary.VLerp` (`self.GetActorScale3D`) (0.0 0.0 0.0) Alpha)))

(fn `TransformAnimation`
  (params (self2 :type "Actor Object Reference") (A :type "Vector Structure") (Alpha :type "Float (double-precision)"))
  (returns (ReturnValue :type "Vector Structure"))
  (return (`KismetMathLibrary.VLerp` A (`self.K2_GetActorLocation` self2) Alpha)))

(fn `UserConstructionScript`)

(fn `Wsysanko`
  (params (PlayerLocation :type "Vector Structure") (NewObjectScale :type "Vector Structure") (Light :type "LightComponent Object Reference") (LightIntensity :type "Float (double-precision)"))
  (`self.K2_SetActorLocation` PlayerLocation)
  (`self.SetActorScale3D` NewObjectScale)
  (`LightComponent.SetIntensity` Light LightIntensity))