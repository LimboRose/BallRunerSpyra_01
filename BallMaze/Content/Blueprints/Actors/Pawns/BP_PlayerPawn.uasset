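; Player pawn for a rolling ball that restarts the level when it takes any damage.
; Left/Right input applies torque to the Ball as an acceleration change, scaled by a multiplier on both X and Y, while Forward/Backwards input has no logic.
; AnyDamage calls LevelRestart, which fades the camera out, waits for the fade to finish and reopens the current level by name.
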(event `InputAxis|Move Forward/Backwards`
  (params (AxisValue :type "Float (single-precision)"))
  ;[1 1 1] Movement
)

(event `InputAxis|Move Left/Right`
  (params (AxisValue :type "Float (single-precision)"))
  (bind _multiplier (`self.Multiplier`))
  ;[1 1 1] Movement
  (`PrimitiveComponent.AddTorqueInRadians` (`self.Ball`) (`KismetMathLibrary.MakeVector` (* AxisValue _multiplier) (* (stale `InputAxis|Move Forward/Backwards` AxisValue) _multiplier)) "None" true))

(event `self.ReceiveAnyDamage`
  (params (Damage :type "Float (single-precision)") (DamageType :type "DamageType Object Reference") (InstigatedBy :type "Controller Object Reference") (DamageCauser :type "Actor Object Reference"))
  ;[1 1 1] DamageSystem
  (`self.LevelRestart`))

(fn `UserConstructionScript`)